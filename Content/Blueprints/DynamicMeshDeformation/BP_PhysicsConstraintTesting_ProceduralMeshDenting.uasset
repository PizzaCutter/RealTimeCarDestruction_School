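; Test car actor (Z3) that combines breakable physics-constrained doors, hood and trunk lid with runtime mesh denting.
; On BeginPlay it links each BP_RuntimeMeshDenting child actor to its static mesh, covering the body and four moving parts.
; A broken constraint switches that part's collision profile to Vehicle.
; ExplodeCar applies a velocity-change radial impulse from the body to nearby static mesh components, excluding the body itself.
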(event OnConstraintBroken(Constraint_Trunk_Lid)
  (params (ConstraintIndex :type Integer))
  (Collision|SetCollisionProfileName (Variables|Default|GetZ3_MovingParts_Z3_Trunk_Lid) "Vehicle" :!class /Script/Engine.PrimitiveComponent))

(event OnConstraintBroken(PhysicsConstraint)
  (params (ConstraintIndex :type Integer))
  (Collision|SetCollisionProfileName (Variables|Default|GetZ3_MovingParts_Z3_Hood) "Vehicle" :!class /Script/Engine.PrimitiveComponent))

(event OnConstraintBroken(Constraint_Right_Door)
  (params (ConstraintIndex :type Integer))
  (Collision|SetCollisionProfileName (Variables|Default|GetZ3_MovingParts_Z3_Right_Door) "Vehicle" :!class /Script/Engine.PrimitiveComponent))

(event OnConstraintBroken(Constraint_Left_Door)
  (params (ConstraintIndex :type Integer))
  (Collision|SetCollisionProfileName (Variables|Default|GetZ3_MovingParts_Z3_left_door) "Vehicle" :!class /Script/Engine.PrimitiveComponent))

(event EventBeginPlay
  (CallFunction|AssignStaticMeshestoProceduralMeshes))

(fn ConstructionScript
  (Utilities|FlowControl|Sequence
    (:then_0
      (Utilities|Array|Clear (Variables|Default|GetPhysicsMeshes))
      (Utilities|FlowControl|Sequence
        (:then_0
          (Utilities|Array|Add (Variables|Default|GetPhysicsMeshes) (Variables|Default|GetZ3_MovingParts_Z3_left_door)))
        (:then_1
          (Utilities|Array|Add (Variables|Default|GetPhysicsMeshes) (Variables|Default|GetZ3_MovingParts_Z3_Right_Door)))
        (:then_2
          (Utilities|Array|Add (Variables|Default|GetPhysicsMeshes) (Variables|Default|GetZ3_MovingParts_Z3_Hood)))
        (:then_3
          (Utilities|Array|Add (Variables|Default|GetPhysicsMeshes) (Variables|Default|GetZ3_MovingParts_Z3_Trunk_Lid)))))))

(fn AssignStaticMeshestoProceduralMeshes
  (Utilities|FlowControl|Sequence
    (:then_0
      (bind _asbp_runtime_mesh_denting (Utilities|Casting|CastToBP_RuntimeMeshDenting (Variables|/Script/Engine.ChildActorComponent|GetChildActor (Variables|Default|GetBP_Z3_MovingParts_Z3_Trunk_Lid))))
      (Class|RuntimeMeshDenting|SetStaticMeshParent _asbp_runtime_mesh_denting (Variables|Default|GetZ3_MovingParts_Z3_Trunk_Lid)))
    (:then_1
      (bind _asbp_runtime_mesh_denting_2 (Utilities|Casting|CastToBP_RuntimeMeshDenting (Variables|/Script/Engine.ChildActorComponent|GetChildActor (Variables|Default|GetBP_Z3_MovingParts_Z3_Right_Door))))
      (Class|RuntimeMeshDenting|SetStaticMeshParent _asbp_runtime_mesh_denting_2 (Variables|Default|GetZ3_MovingParts_Z3_Right_Door)))
    (:then_2
      (bind _asbp_runtime_mesh_denting_3 (Utilities|Casting|CastToBP_RuntimeMeshDenting (Variables|/Script/Engine.ChildActorComponent|GetChildActor (Variables|Default|GetBP_Z3_MovingParts_Z3_Hood))))
      (Class|RuntimeMeshDenting|SetStaticMeshParent _asbp_runtime_mesh_denting_3 (Variables|Default|GetZ3_MovingParts_Z3_Hood)))
    (:then_3
      (bind _asbp_runtime_mesh_denting_4 (Utilities|Casting|CastToBP_RuntimeMeshDenting (Variables|/Script/Engine.ChildActorComponent|GetChildActor (Variables|Default|GetBP_Z3_MovingParts_Z3_left_door))))
      (Class|RuntimeMeshDenting|SetStaticMeshParent _asbp_runtime_mesh_denting_4 (Variables|Default|GetZ3_MovingParts_Z3_left_door)))
    (:then_4
      (bind _asbp_runtime_mesh_denting_5 (Utilities|Casting|CastToBP_RuntimeMeshDenting (Variables|/Script/Engine.ChildActorComponent|GetChildActor (Variables|Default|GetBP_Z3_MainBody_Z3_Body))))
      (Class|RuntimeMeshDenting|SetStaticMeshParent _asbp_runtime_mesh_denting_5 (Variables|Default|GetZ3_MainBody_Z3_Body)))))

(fn ExplodeCar
  (bind _outcomponents (Collision|SphereOverlapComponents (Transformation|GetWorldLocation (Variables|Default|GetZ3_MainBody_Z3_Body)) 1e+03 (Utilities|Array|MakeArray "ObjectTypeQuery9" "ObjectTypeQuery5") "/Script/Engine.StaticMeshComponent"))
  (for _array_element _outcomponents
    (if (!= _array_element (Variables|Default|GetZ3_MainBody_Z3_Body))
      (Physics|AddRadialImpulse _array_element (Transformation|GetWorldLocation (Variables|Default|GetZ3_MainBody_Z3_Body)) 1e+03 3e+03 "RIF_Linear" true))))