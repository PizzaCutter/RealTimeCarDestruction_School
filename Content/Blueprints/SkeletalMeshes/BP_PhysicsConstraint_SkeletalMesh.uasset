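; Physics constraint test Blueprint for a Z3 car that throws open its hood, doors and trunk lid with impulses.
; Two seconds after BeginPlay, each part receives a velocity-change impulse scaled by ForceAmount, upward for hood and trunk, sideways for doors.
; Every tick, SKZ3MovingPartHood copies the simulated hood's relative rotation and snaps to HoodTest's world location using teleport moves.
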(event EventBeginPlay
  (Utilities|FlowControl|Delay 2.0)
  (Physics|AddImpulse (Variables|Default|GetZ3_MovingPart_Hood) (* "0,0.000000,1.000000" (Variables|Default|GetForceAmount)) "None" true)
  (Physics|AddImpulse (Variables|Default|GetZ3_MovingParts_Z3_Right_Door) (* "0,-1.000000,0.000000" (Variables|Default|GetForceAmount)) "None" true)
  (Physics|AddImpulse (Variables|Default|GetZ3_MovingParts_Z3_Trunk_Lid) (* "0,0.000000,1.000000" (Variables|Default|GetForceAmount)) "None" true)
  (Physics|AddImpulse (Variables|Default|GetZ3_MovingParts_Z3_left_door) (* "0,1.000000, 0" (Variables|Default|GetForceAmount)) "None" true))

(event EventTick
  (params (DeltaSeconds :type Float%20%28single-precision%29))
  (Transformation|SetRelativeRotation (Variables|Default|GetSK_Z3_MovingPart_Hood) (Variables|/Script/Engine.SceneComponent|GetRelativeRotation (Variables|Default|GetZ3_MovingPart_Hood)) false true)
  (Transformation|SetWorldLocation (Variables|Default|GetSK_Z3_MovingPart_Hood) (Transformation|GetWorldLocation (Variables|Default|Gethood_test)) false true))

(fn ConstructionScript)