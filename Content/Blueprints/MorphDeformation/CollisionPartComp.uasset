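; Collision part component that deforms a target mesh through morph targets as it takes impacts.
; OnHit ignores impulses below MinimumVelocity and normalizes stronger ones against MaximumVelocity, without yet accounting for object mass.
; ApplyDamage accumulates clamped Damage, then adds that running total, scaled by each connection's Influence, onto the current morph weight, so deformation compounds with every hit.
; BeginPlay keeps MaximumVelocity from falling below the minimum.
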(event EventBeginPlay
  (CallFunction|VelocityCheck))

(fn VelocityCheck
  (if (< (Variables|Default|GetMaximumVelocity) (Variables|Default|GetMinimumVelocity))
    (Variables|Default|SetMaximumVelocity (Variables|Default|GetMinimumVelocity))))

(fn OnHit
  (params (Hit%20Comp :type Primitive%20Component%20Object%20Reference) (Other%20Actor :type Actor%20Object%20Reference) (Other%20Comp :type Actor%20Component%20Object%20Reference) (Normal%20Impulse :type Vector) (Hit%20Result :type Hit%20Result%20Structure))
  (LocalVariables|SetL_NormalImpulse Normal%20Impulse)
  (LocalVariables|SetL_NormalImpulseLength (Math|Vector|VectorLength Normal%20Impulse))
  ;[1 1 1] false if the impact is to low to do damage
  (if (>= (LocalVariables|GetL_NormalImpulseLength) (Variables|Default|GetMinimumVelocity))
    (Utilities|FlowControl|Sequence
      (:then_0
        ;[1 0 0] TODO-TAKE IN ACCOUNT OBJECT MASS
        ;;[1 1 1] Calculate damage the impact has to do
        (if (< (LocalVariables|GetL_NormalImpulseLength) (Variables|Default|GetMaximumVelocity))
          ;;;[1 1 1] Calculate damage based on velocity
          (LocalVariables|SetL_NormalizedDamage (/ (LocalVariables|GetL_NormalImpulseLength) (Variables|Default|GetMaximumVelocity)))
          (else
            (LocalVariables|SetL_NormalizedDamage 1.0))))
      (:then_2
        (CallFunction|ApplyDamage (LocalVariables|GetL_NormalizedDamage))))))

(fn ApplyDamage
  (params (NormalizedIncomingDamage :type Float%20%28single-precision%29))
  (bind _targetmesh (Variables|Default|GetTargetMesh))
  (Variables|Default|SetDamage (Math|Float|Clamp(Float) (+ NormalizedIncomingDamage (Variables|Default|GetDamage))))
  (for _array_element (Variables|Default|GetConnections)
    (Components|SkeletalMesh|SetMorphTarget _targetmesh (.morphtargetconnection _array_element) (Math|Float|Clamp(Float) (+ (Class|SkeletalMeshComponent|GetMorphTarget _targetmesh (.morphtargetconnection _array_element)) (* (.influence _array_element) (Variables|Default|GetDamage))) -1.0) true)))