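; Deformable actor that routes impacts on box damage volumes into morph-target damage and swaps its collision to match.
; Overlaps on front, back, top and frontal volumes call OnHit on the matching part component, passing the other actor's velocity as impulse.
; Each tick, noticeable changes in the Frontal_Collision_Damage morph select NoDamage or MaxDamage body collider and impact volumes at a half-damage threshold.
; Initialization links part components to the skeletal mesh and caches both volume sets.
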(event OnComponentBeginOverlap(1_Front_Right_Collider)
  (params (OverlappedComponent :type Primitive%20Component%20Object%20Reference) (OtherActor :type Actor%20Object%20Reference) (OtherComp :type Primitive%20Component%20Object%20Reference) (OtherBodyIndex :type Integer) (bFromSweep :type Boolean) (SweepResult :type Hit%20Result%20Structure%20%28by%20ref%29))
  (Default|OnHit (Variables|Default|GetFront_Right_Comp) OverlappedComponent OtherActor OtherComp (Transformation|GetVelocity OtherActor) SweepResult))

(event OnComponentBeginOverlap(1_Frontal_Collision_Collider)
  (params (OverlappedComponent :type Primitive%20Component%20Object%20Reference) (OtherActor :type Actor%20Object%20Reference) (OtherComp :type Primitive%20Component%20Object%20Reference) (OtherBodyIndex :type Integer) (bFromSweep :type Boolean) (SweepResult :type Hit%20Result%20Structure%20%28by%20ref%29))
  (Default|OnHit (Variables|Default|GetFrontal_Collision_Comp) OverlappedComponent OtherActor OtherComp (Transformation|GetVelocity OtherActor) SweepResult))

(event OnComponentBeginOverlap(1_Top_Center_Collider)
  (params (OverlappedComponent :type Primitive%20Component%20Object%20Reference) (OtherActor :type Actor%20Object%20Reference) (OtherComp :type Primitive%20Component%20Object%20Reference) (OtherBodyIndex :type Integer) (bFromSweep :type Boolean) (SweepResult :type Hit%20Result%20Structure%20%28by%20ref%29))
  (Default|OnHit (Variables|Default|GetTop_Center_Comp) OverlappedComponent OtherActor OtherComp (Transformation|GetVelocity OtherActor) SweepResult))

(event OnComponentBeginOverlap(2_Frontal_Collision_Collider)
  (params (OverlappedComponent :type Primitive%20Component%20Object%20Reference) (OtherActor :type Actor%20Object%20Reference) (OtherComp :type Primitive%20Component%20Object%20Reference) (OtherBodyIndex :type Integer) (bFromSweep :type Boolean) (SweepResult :type Hit%20Result%20Structure%20%28by%20ref%29))
  (Default|OnHit (Variables|Default|GetFrontal_Collision_Comp) OverlappedComponent OtherActor OtherComp (Transformation|GetVelocity OtherActor) SweepResult))

(event OnComponentBeginOverlap(2_Front_Left_Collider)
  (params (OverlappedComponent :type Primitive%20Component%20Object%20Reference) (OtherActor :type Actor%20Object%20Reference) (OtherComp :type Primitive%20Component%20Object%20Reference) (OtherBodyIndex :type Integer) (bFromSweep :type Boolean) (SweepResult :type Hit%20Result%20Structure%20%28by%20ref%29))
  (Default|OnHit (Variables|Default|GetFront_Left_Comp) OverlappedComponent OtherActor OtherComp (Transformation|GetVelocity OtherActor) SweepResult))

(event OnComponentBeginOverlap(2_Front_Right_Collider)
  (params (OverlappedComponent :type Primitive%20Component%20Object%20Reference) (OtherActor :type Actor%20Object%20Reference) (OtherComp :type Primitive%20Component%20Object%20Reference) (OtherBodyIndex :type Integer) (bFromSweep :type Boolean) (SweepResult :type Hit%20Result%20Structure%20%28by%20ref%29))
  (Default|OnHit (Variables|Default|GetFront_Right_Comp) OverlappedComponent OtherActor OtherComp (Transformation|GetVelocity OtherActor) SweepResult))

(event OnComponentBeginOverlap(2_Back_Right_Collider_01)
  (params (OverlappedComponent :type Primitive%20Component%20Object%20Reference) (OtherActor :type Actor%20Object%20Reference) (OtherComp :type Primitive%20Component%20Object%20Reference) (OtherBodyIndex :type Integer) (bFromSweep :type Boolean) (SweepResult :type Hit%20Result%20Structure%20%28by%20ref%29))
  (Default|OnHit (Variables|Default|GetBack_Right_Comp) OverlappedComponent OtherActor OtherComp (Transformation|GetVelocity OtherActor) SweepResult))

(event OnComponentBeginOverlap(2_Back_Right_Collider_02)
  (params (OverlappedComponent :type Primitive%20Component%20Object%20Reference) (OtherActor :type Actor%20Object%20Reference) (OtherComp :type Primitive%20Component%20Object%20Reference) (OtherBodyIndex :type Integer) (bFromSweep :type Boolean) (SweepResult :type Hit%20Result%20Structure%20%28by%20ref%29))
  (Default|OnHit (Variables|Default|GetBack_Right_Comp) OverlappedComponent OtherActor OtherComp (Transformation|GetVelocity OtherActor) SweepResult))

(event OnComponentBeginOverlap(2_Back_Left_Collider_01)
  (params (OverlappedComponent :type Primitive%20Component%20Object%20Reference) (OtherActor :type Actor%20Object%20Reference) (OtherComp :type Primitive%20Component%20Object%20Reference) (OtherBodyIndex :type Integer) (bFromSweep :type Boolean) (SweepResult :type Hit%20Result%20Structure%20%28by%20ref%29))
  (Default|OnHit (Variables|Default|GetBack_Left_Comp) OverlappedComponent OtherActor OtherComp (Transformation|GetVelocity OtherActor) SweepResult))

(event OnComponentBeginOverlap(2_Back_Left_Collider_02)
  (params (OverlappedComponent :type Primitive%20Component%20Object%20Reference) (OtherActor :type Actor%20Object%20Reference) (OtherComp :type Primitive%20Component%20Object%20Reference) (OtherBodyIndex :type Integer) (bFromSweep :type Boolean) (SweepResult :type Hit%20Result%20Structure%20%28by%20ref%29))
  (Default|OnHit (Variables|Default|GetBack_Left_Comp) OverlappedComponent OtherActor OtherComp (Transformation|GetVelocity OtherActor) SweepResult))

(event OnComponentBeginOverlap(2_Top_Center_Collider)
  (params (OverlappedComponent :type Primitive%20Component%20Object%20Reference) (OtherActor :type Actor%20Object%20Reference) (OtherComp :type Primitive%20Component%20Object%20Reference) (OtherBodyIndex :type Integer) (bFromSweep :type Boolean) (SweepResult :type Hit%20Result%20Structure%20%28by%20ref%29))
  (Default|OnHit (Variables|Default|GetTop_Center_Comp) OverlappedComponent OtherActor OtherComp (Transformation|GetVelocity OtherActor) SweepResult))

(event OnComponentBeginOverlap(1_Front_Left_Collider)
  (params (OverlappedComponent :type Primitive%20Component%20Object%20Reference) (OtherActor :type Actor%20Object%20Reference) (OtherComp :type Primitive%20Component%20Object%20Reference) (OtherBodyIndex :type Integer) (bFromSweep :type Boolean) (SweepResult :type Hit%20Result%20Structure%20%28by%20ref%29))
  (Default|OnHit (Variables|Default|GetFront_Left_Comp) OverlappedComponent OtherActor OtherComp (Transformation|GetVelocity OtherActor) SweepResult))

(event OnComponentBeginOverlap(1_Back_Left_Collider)
  (params (OverlappedComponent :type Primitive%20Component%20Object%20Reference) (OtherActor :type Actor%20Object%20Reference) (OtherComp :type Primitive%20Component%20Object%20Reference) (OtherBodyIndex :type Integer) (bFromSweep :type Boolean) (SweepResult :type Hit%20Result%20Structure%20%28by%20ref%29))
  (Default|OnHit (Variables|Default|GetBack_Left_Comp) OverlappedComponent OtherActor OtherComp (Transformation|GetVelocity OtherActor) SweepResult))

(event OnComponentBeginOverlap(1_Back_Right_Collider)
  (params (OverlappedComponent :type Primitive%20Component%20Object%20Reference) (OtherActor :type Actor%20Object%20Reference) (OtherComp :type Primitive%20Component%20Object%20Reference) (OtherBodyIndex :type Integer) (bFromSweep :type Boolean) (SweepResult :type Hit%20Result%20Structure%20%28by%20ref%29))
  (Default|OnHit (Variables|Default|GetBack_Right_Comp) OverlappedComponent OtherActor OtherComp (Transformation|GetVelocity OtherActor) SweepResult))

(event EventBeginPlay
  (CallFunction|Initialize))

(event EventTick
  (params (DeltaSeconds :type Float%20%28single-precision%29))
  (CallFunction|UpdateCollision))

(fn ConstructionScript)

(fn Initialize
  (Utilities|FlowControl|Sequence
    (:then_0
      ;[1 1 1] Assign the skeletal mesh to each collision part component
      (for _array_element (Actor|GetComponentsByClass "/Game/Blueprints/MorphDeformation/CollisionPartComp.CollisionPartComp_C")
        (Variables|/Game/Blueprints/MorphDeformation/CollisionPartComp.CollisionPartComp_C|SetTargetMesh _array_element (Variables|Default|GetSkeletalMesh))))
    (:then_1
      ;[1 1 1] Find All Colliders needed for impact locations for the NoDamage tier
      (Utilities|Array|Clear (Variables|Default|GetNoDamageImpactLocationsArr))
      (for _array_element_2 (Components|GetChildrenComponents (Variables|Default|GetNoDamageImpactLocations) true)
        (bind _asbox_collision (Utilities|Casting|CastToBoxComponent _array_element_2))
        (Utilities|Array|Add (Variables|Default|GetNoDamageImpactLocationsArr) _asbox_collision)))
    (:then_2
      ;[1 1 1] Find all colliders needed for impact locations for the MaxDamage tier
      (Utilities|Array|Clear (Variables|Default|GetMaxDamageImpactLocationsArr))
      (for _array_element_3 (Components|GetChildrenComponents (Variables|Default|GetMaxDamageImpactLocations) true)
        (bind _asbox_collision_2 (Utilities|Casting|CastToBoxComponent _array_element_3))
        (Utilities|Array|Add (Variables|Default|GetMaxDamageImpactLocationsArr) _asbox_collision_2)))))

(fn ResetMorphTargets
  (for _array_element (Variables|Blending|GetMorphTargets)
    (Components|SkeletalMesh|SetMorphTarget (Variables|Default|GetSkeletalMesh) _array_element 0.0 true)))

(fn UpdateCollision
  (Utilities|FlowControl|Sequence
    (:then_0
      (LocalVariables|SetL_CurMorphTarget (Class|SkeletalMeshComponent|GetMorphTarget (Variables|Default|GetSkeletalMesh) "Frontal_Collision_Damage"))
      (if (not (Math|Float|NearlyEqual(Float) (Variables|Default|GetPrevMorphTarget) (LocalVariables|GetL_CurMorphTarget) 0.05))
        ;[1 1 1] We now have more then 50% damage so toggle to different collision
        (if (>= (LocalVariables|GetL_CurMorphTarget) 0.5)
          (Collision|SetCollisionEnabled (Variables|Default|GetNoDamage_Collider_01) "NoCollision")
          (Collision|SetCollisionEnabled (Variables|Default|GetMaxDamage_Collider_01) "QueryAndPhysics")
          ;[1 1 1] Update the impact locations that are being used
          (CallFunction|ToggleCollisiononArray (Variables|Default|GetNoDamageImpactLocationsArr) "NoCollision")
          (CallFunction|ToggleCollisiononArray (Variables|Default|GetMaxDamageImpactLocationsArr) "QueryOnly")
          (else
            (Collision|SetCollisionEnabled (Variables|Default|GetNoDamage_Collider_01) "QueryAndPhysics")
            (Collision|SetCollisionEnabled (Variables|Default|GetMaxDamage_Collider_01) "NoCollision")
            (CallFunction|ToggleCollisiononArray (Variables|Default|GetNoDamageImpactLocationsArr) "QueryOnly")
            (CallFunction|ToggleCollisiononArray (Variables|Default|GetMaxDamageImpactLocationsArr) "NoCollision")))))
    (:then_1
      (Variables|Default|SetPrevMorphTarget (LocalVariables|GetL_CurMorphTarget)))))

(fn ToggleCollisiononArray
  (params (Arr :type Array%20of%20Box%20Component%20Object%20References) (NewState :type ECollisionEnabled%20Enum :default "NoCollision"))
  (for _array_element Arr
    (Collision|SetCollisionEnabled _array_element NewState)))