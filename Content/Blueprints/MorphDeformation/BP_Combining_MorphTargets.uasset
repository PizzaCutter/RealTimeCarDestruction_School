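; Demo actor that cycles a skeletal mesh through a list of morph targets, then plays them all combined.
; Tick ramps a value up and down, normalized by a period, as the weight of the current target.
; Looping timers flip the ramp direction every period and advance the target index every two periods.
; An index equal to the array length drives all targets together; the next step resets weights and restarts.
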(event Custom|IncrementIndex
  (bind _result (Math|Integer|IncrementInt (Variables|Blending|GetCurMorphTargetIndex))
    (:%20%20
      (if (> _result (Utilities|Array|Length (Variables|Blending|GetMorphTargets)))
        (Variables|Blending|SetCurMorphTargetIndex 0)
        (CallFunction|ResetMorphTargets)))))

(event Custom|FlipFlop
  (Variables|FlipFlop|SetUp (not (Variables|FlipFlop|GetUp))))

(event EventBeginPlay
  (CallFunction|Initialize)
  (Utilities|Time|SetTimerbyEvent (delegate Custom|FlipFlop) (Variables|FlipFlop|GetTime) true)
  (Utilities|Time|SetTimerbyEvent (delegate Custom|IncrementIndex) (* (Variables|FlipFlop|GetTime) 2.0) true))

(event EventTick
  (params (DeltaSeconds :type Float%20%28single-precision%29))
  (CallFunction|UpdateTimer)
  (CallFunction|UpdateMorphTargets))

(fn ConstructionScript)

(fn Initialize)

(fn UpdateMorphTargets
  (if (== (Variables|Blending|GetCurMorphTargetIndex) (Utilities|Array|Length (Variables|Blending|GetMorphTargets)))
    (for _array_element (Variables|Blending|GetMorphTargets)
      (Components|SkeletalMesh|SetMorphTarget (Variables|Default|GetSkeletalMesh) _array_element (/ (Variables|FlipFlop|GetTimer) (Variables|FlipFlop|GetTime)) true))
    (else
      (Components|SkeletalMesh|SetMorphTarget (Variables|Default|GetSkeletalMesh) (Utilities|Array|Get(acopy) (Variables|Blending|GetMorphTargets) (Variables|Blending|GetCurMorphTargetIndex)) (/ (Variables|FlipFlop|GetTimer) (Variables|FlipFlop|GetTime)) true))))

(fn UpdateTimer
  (if (Variables|FlipFlop|GetUp)
    (Variables|FlipFlop|SetTimer (+ (Variables|FlipFlop|GetTimer) (Utilities|Time|GetWorldDeltaSeconds)))
    (else
      (Variables|FlipFlop|SetTimer (- (Variables|FlipFlop|GetTimer) (Utilities|Time|GetWorldDeltaSeconds))))))

(fn ResetMorphTargets
  (for _array_element (Variables|Blending|GetMorphTargets)
    (Components|SkeletalMesh|SetMorphTarget (Variables|Default|GetSkeletalMesh) _array_element 0.0 true)))