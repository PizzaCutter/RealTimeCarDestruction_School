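; Actor Blueprint that shows progressive frontal collision damage on a skeletal mesh through a morph target.
; The Frontal_Collision_Damage morph starts at zero on BeginPlay.
; Each component hit destroys the other actor, increments a Timer variable and applies it as the morph weight.
; Despite its name, Timer counts hits rather than time, and Tick resets it once it passes a cap, without updating the morph.
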(event OnComponentHit(SkeletalMesh)
  (params (HitComponent :type Primitive%20Component%20Object%20Reference) (OtherActor :type Actor%20Object%20Reference) (OtherComp :type Primitive%20Component%20Object%20Reference) (NormalImpulse :type Vector :default "0, 0, 0") (Hit :type Hit%20Result%20Structure%20%28by%20ref%29))
  (Actor|DestroyActor OtherActor)
  (bind _output_get (Variables|Default|SetTimer (+ (Variables|Default|GetTimer) 0.1)))
  (Components|SkeletalMesh|SetMorphTarget (Variables|Default|GetSkeletalMesh) "Frontal_Collision_Damage" _output_get true))

(event EventBeginPlay
  (Components|SkeletalMesh|SetMorphTarget (Variables|Default|GetSkeletalMesh) "Frontal_Collision_Damage" 0.0 true))

(event EventTick
  (params (DeltaSeconds :type Float%20%28single-precision%29))
  (if (> (Variables|Default|GetTimer) 1.5)
    (Variables|Default|SetTimer 0.0)))

(fn ConstructionScript)