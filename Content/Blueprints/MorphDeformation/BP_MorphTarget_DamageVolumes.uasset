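; Skeletal mesh actor with damage volumes around its front, rear corners and top, set up for morph target deformation on impact.
; Each of the six colliders forwards its hit events to a matching part component, which holds the per-region response.
; On BeginPlay every CollisionPartComp receives the skeletal mesh as its target.
; ResetMorphTargets zeroes each morph target in the MorphTargets list to clear deformation.
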(event OnComponentHit(Front_Left_Collider)
  (params (HitComponent :type Primitive%20Component%20Object%20Reference) (OtherActor :type Actor%20Object%20Reference) (OtherComp :type Primitive%20Component%20Object%20Reference) (NormalImpulse :type Vector :default "0, 0, 0") (Hit :type Hit%20Result%20Structure%20%28by%20ref%29))
  (Default|OnHit (Variables|Default|GetFront_Left_Comp) HitComponent OtherActor OtherComp NormalImpulse Hit))

(event OnComponentHit(Back_Left_Collider)
  (params (HitComponent :type Primitive%20Component%20Object%20Reference) (OtherActor :type Actor%20Object%20Reference) (OtherComp :type Primitive%20Component%20Object%20Reference) (NormalImpulse :type Vector :default "0, 0, 0") (Hit :type Hit%20Result%20Structure%20%28by%20ref%29))
  (Default|OnHit (Variables|Default|GetBack_Left_Comp) HitComponent OtherActor OtherComp NormalImpulse Hit))

(event OnComponentHit(Back_Right_Collider)
  (params (HitComponent :type Primitive%20Component%20Object%20Reference) (OtherActor :type Actor%20Object%20Reference) (OtherComp :type Primitive%20Component%20Object%20Reference) (NormalImpulse :type Vector :default "0, 0, 0") (Hit :type Hit%20Result%20Structure%20%28by%20ref%29))
  (Default|OnHit (Variables|Default|GetBack_Right_Comp) HitComponent OtherActor OtherComp NormalImpulse Hit))

(event OnComponentHit(Front_Right_Collider)
  (params (HitComponent :type Primitive%20Component%20Object%20Reference) (OtherActor :type Actor%20Object%20Reference) (OtherComp :type Primitive%20Component%20Object%20Reference) (NormalImpulse :type Vector :default "0, 0, 0") (Hit :type Hit%20Result%20Structure%20%28by%20ref%29))
  (Default|OnHit (Variables|Default|GetFront_Right_Comp) HitComponent OtherActor OtherComp NormalImpulse Hit))

(event OnComponentHit(Frontal_Collision_Collider)
  (params (HitComponent :type Primitive%20Component%20Object%20Reference) (OtherActor :type Actor%20Object%20Reference) (OtherComp :type Primitive%20Component%20Object%20Reference) (NormalImpulse :type Vector :default "0, 0, 0") (Hit :type Hit%20Result%20Structure%20%28by%20ref%29))
  (Default|OnHit (Variables|Default|GetFrontal_Collision_Comp) HitComponent OtherActor OtherComp NormalImpulse Hit))

(event OnComponentHit(Top_Center_Collider)
  (params (HitComponent :type Primitive%20Component%20Object%20Reference) (OtherActor :type Actor%20Object%20Reference) (OtherComp :type Primitive%20Component%20Object%20Reference) (NormalImpulse :type Vector :default "0, 0, 0") (Hit :type Hit%20Result%20Structure%20%28by%20ref%29))
  (Default|OnHit (Variables|Default|GetTop_Center_Comp) HitComponent OtherActor OtherComp NormalImpulse Hit))

(event EventBeginPlay
  (CallFunction|Initialize))

(fn ConstructionScript)

(fn Initialize
  (for _array_element (Actor|GetComponentsByClass "/Game/Blueprints/MorphDeformation/CollisionPartComp.CollisionPartComp_C")
    (Variables|/Game/Blueprints/MorphDeformation/CollisionPartComp.CollisionPartComp_C|SetTargetMesh _array_element (Variables|Default|GetSkeletalMesh))))

(fn ResetMorphTargets
  (for _array_element (Variables|Blending|GetMorphTargets)
    (Components|SkeletalMesh|SetMorphTarget (Variables|Default|GetSkeletalMesh) _array_element 0.0 true)))