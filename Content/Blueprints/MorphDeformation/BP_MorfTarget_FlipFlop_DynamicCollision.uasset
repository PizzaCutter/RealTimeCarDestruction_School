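; Actor that ping-pongs a skeletal mesh's frontal collision damage morph target and swaps its collision boxes to match the deformation.
; A looping timer flips the direction, while Tick ramps a time value up or down to drive the morph weight.
; BeginPlay caches the box children of the NoDamage and MaxDamage components.
; Every Tick enables the full-damage set from the halfway point onward, otherwise the no-damage set, disabling the other.
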(event Custom|CustomEvent_0
  (Variables|Default|SetUp (not (Variables|Default|GetUp))))

(event EventBeginPlay
  (Utilities|Time|SetTimerbyEvent (delegate Custom|CustomEvent_0) (Variables|Default|GetTime) true)
  (Utilities|FlowControl|Sequence
    (:then_0
      ;[1 1 1] Get all No Damage Colliders
      (for _array_element (Components|GetChildrenComponents (Variables|Default|GetNoDamage) false)
        (bind _asbox_collision (Utilities|Casting|CastToBoxComponent _array_element))
        (Utilities|Array|Add (Variables|Default|GetNoDamageColliders) _asbox_collision)))
    (:then_1
      ;[1 1 1] Get all full damage colliders
      (for _array_element_2 (Components|GetChildrenComponents (Variables|Default|GetMaxDamage) false)
        (bind _asbox_collision_2 (Utilities|Casting|CastToBoxComponent _array_element_2))
        (Utilities|Array|Add (Variables|Default|GetFullDamageCollider) _asbox_collision_2)))))

(event EventTick
  (params (DeltaSeconds :type Float%20%28single-precision%29))
  (Utilities|FlowControl|Sequence
    (:then_0
      (if (Variables|Default|GetUp)
        (Variables|Default|SetTimer (+ (Variables|Default|GetTimer) (Utilities|Time|GetWorldDeltaSeconds)))
        (else
          (Variables|Default|SetTimer (- (Variables|Default|GetTimer) (Utilities|Time|GetWorldDeltaSeconds))))))
    (:then_1
      (Components|SkeletalMesh|SetMorphTarget (Variables|Default|GetSkeletalMesh) "Frontal_Collision_Damage" (/ (Variables|Default|GetTimer) (Variables|Default|GetTime)) true))
    (:then_2
      (if (>= (Variables|Default|GetTimer) (/ (Variables|Default|GetTime) 2.0))
        (CallFunction|SetFullDamageCollision true)
        (CallFunction|SetNoDamageCollision false)
        (else
          (CallFunction|SetFullDamageCollision false)
          (CallFunction|SetNoDamageCollision true))))))

(fn ConstructionScript)

(fn SetNoDamageCollision
  (params (NewState :type Boolean))
  (if NewState
    (for _array_element (Variables|Default|GetNoDamageColliders)
      (Collision|SetCollisionEnabled _array_element "QueryAndPhysics"))
    (else
      (for _array_element_2 (Variables|Default|GetNoDamageColliders)
        (Collision|SetCollisionEnabled _array_element_2 "NoCollision")))))

(fn SetFullDamageCollision
  (params (NewState :type Boolean))
  (if NewState
    (for _array_element (Variables|Default|GetFullDamageCollider)
      (Collision|SetCollisionEnabled _array_element "QueryAndPhysics"))
    (else
      (for _array_element_2 (Variables|Default|GetFullDamageCollider)
        (Collision|SetCollisionEnabled _array_element_2 "NoCollision")))))