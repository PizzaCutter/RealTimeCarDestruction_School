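; Actor Blueprint that continuously oscillates the Frontal_Collision_Damage morph target on its skeletal mesh, animating the deformation back and forth.
; A looping timer, started on BeginPlay with period Time, flips the Up flag.
; Tick adds or subtracts delta seconds from Timer according to Up, then applies Timer divided by Time as the morph weight, without clamping.
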(event Custom|CustomEvent_0
  (Variables|Default|SetUp (not (Variables|Default|GetUp))))

(event EventBeginPlay
  (Utilities|Time|SetTimerbyEvent (delegate Custom|CustomEvent_0) (Variables|Default|GetTime) true))

(event EventTick
  (params (DeltaSeconds :type Float%20%28single-precision%29))
  (Utilities|FlowControl|Sequence
    (:then_0
      (if (Variables|Default|GetUp)
        (Variables|Default|SetTimer (+ (Variables|Default|GetTimer) (Utilities|Time|GetWorldDeltaSeconds)))
        (else
          (Variables|Default|SetTimer (- (Variables|Default|GetTimer) (Utilities|Time|GetWorldDeltaSeconds))))))
    (:then_1
      (Components|SkeletalMesh|SetMorphTarget (Variables|Default|GetSkeletalMesh) "Frontal_Collision_Damage" (/ (Variables|Default|GetTimer) (Variables|Default|GetTime)) true))))

(fn ConstructionScript)