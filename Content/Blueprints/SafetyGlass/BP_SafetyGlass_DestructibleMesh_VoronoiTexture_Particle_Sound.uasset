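; Safety glass pane that cracks visually under hits, then swaps to a destructible mesh at a damage limit.
; At BeginPlay it creates brush materials and diffuse, normal and crack-mask render targets feeding the pane's dynamic material.
; Each hit traces through the impact to find UVs, stamps randomized brushes into those targets and spawns splinter particles and smash sound.
; Enough hits hide the static mesh and attach a destructible actor carrying the cracked material.
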(event OnComponentHit(StaticMesh)
  (params (HitComponent :type Primitive%20Component%20Object%20Reference) (OtherActor :type Actor%20Object%20Reference) (OtherComp :type Primitive%20Component%20Object%20Reference) (NormalImpulse :type Vector :default "0, 0, 0") (Hit :type Hit%20Result%20Structure%20%28by%20ref%29))
  (CallFunction|ImpactHit OtherActor Hit))

(event EventBeginPlay
  (Init|CreateBrushes)
  (Init|CreateMaterialsforStaticMesh)
  (Init|CreateRenderTargets))

(fn ConstructionScript
  (Components|StaticMesh|SetStaticMesh (Variables|Default|GetStaticMesh) (Variables|Default|GetStaticMeshAsset)))

(fn UpdateBrushTextures
  (bind _brushtextures (Variables|Brush|GetBrushTextures))
  (bind _brushnormaltextures (Variables|Brush|GetBrushNormalTextures))
  (Rendering|Material|SetTextureParameterValue (Variables|Brush|GetGlassBrush) "Decal" (Utilities|Array|Get(acopy) _brushtextures (Math|Random|RandomInteger (Utilities|Array|Length _brushtextures))))
  (Rendering|Material|SetTextureParameterValue (Variables|Brush|GetGlassBrushNormal) "Decal" (Utilities|Array|Get(acopy) _brushnormaltextures (Math|Random|RandomInteger (Utilities|Array|Length _brushnormaltextures)))))

(fn SpawnDestructibleMesh
  (if (not (Variables|DestructibleMeshes|GetHasSpawned))
    (Utilities|FlowControl|Sequence
      (:then_0
        ;[1 1 1] Spawn destructible mesh and assign materials
        (bind _returnvalue (Game|SpawnActorfromClass "/Script/ApexDestruction.DestructibleActor" (Transformation|GetWorldTransform (Variables|Default|GetStaticMesh)) "AlwaysSpawn" 0 0))
        (Transformation|AttachComponentToComponent _returnvalue (Variables|Default|GetStaticMesh) "None" "SnapToTarget" "SnapToTarget" "SnapToTarget" false)
        (Class|DestructibleComponent|SetDestructibleMesh (Variables|/Script/ApexDestruction.DestructibleActor|GetDestructibleComponent _returnvalue) (Variables|DestructibleMeshes|GetDestructibleMesh))
        (Rendering|Material|SetMaterial (Variables|/Script/ApexDestruction.DestructibleActor|GetDestructibleComponent _returnvalue) 0 (Variables|Default|GetMeshMaterial))
        (Rendering|Material|SetMaterial (Variables|/Script/ApexDestruction.DestructibleActor|GetDestructibleComponent _returnvalue) 1 "/Game/Materials/SafetyGlass/M_BaseGlass_Inst.M_BaseGlass_Inst")
        (Variables|DestructibleMeshes|SetHasSpawned true))
      (:then_1
        (Rendering|SetVisibility (Variables|Default|GetStaticMesh) false false)
        (Collision|SetCollisionEnabled (Variables|Default|GetStaticMesh) "NoCollision")))))

(fn CreateBrushes
  ;[1 1 1] Create and cache brush material for diffuse map
  (bind _returnvalue (Rendering|Material|CreateDynamicMaterialInstance "/Game/Materials/SafetyGlass/Brushes/M_GlassBrush.M_GlassBrush" "None" :!class /Script/Engine.KismetMaterialLibrary))
  (bind _output_get (Variables|Brush|SetGlassBrush _returnvalue))
  (Rendering|Material|SetScalarParameterValue _output_get "Size" (Variables|Brush|GetBrushSize) :!class /Script/Engine.MaterialInstanceDynamic)
  ;[1 1 1] Create and cache brush material for normal map
  (bind _returnvalue_2 (Rendering|Material|CreateDynamicMaterialInstance "/Game/Materials/SafetyGlass/Brushes/M_GlassBrushNormal.M_GlassBrushNormal" "None" :!class /Script/Engine.KismetMaterialLibrary))
  (bind _output_get_2 (Variables|Brush|SetGlassBrushNormal _returnvalue_2))
  (Rendering|Material|SetScalarParameterValue _output_get_2 "Size" (Variables|Brush|GetCrackBrushSize) :!class /Script/Engine.MaterialInstanceDynamic)
  ;[1 1 1] Create and cache brush material for normal map
  (bind _returnvalue_3 (Rendering|Material|CreateDynamicMaterialInstance "/Game/Materials/SafetyGlass/Brushes/M_CircleGradientBrush.M_CircleGradientBrush" "None" :!class /Script/Engine.KismetMaterialLibrary))
  (bind _output_get_3 (Variables|Brush|SetCrackBrush _returnvalue_3))
  (Rendering|Material|SetScalarParameterValue _output_get_3 "Size" (Variables|Brush|GetBrushSize) :!class /Script/Engine.MaterialInstanceDynamic))

(fn CreateMaterialsforStaticMesh
  ;[1 1 1] Create and cache a dynamic material
  (bind _returnvalue (Rendering|Material|CreateDynamicMaterialInstance (Rendering|Material|GetMaterial (Variables|Default|GetStaticMesh) 0) "None" :!class /Script/Engine.KismetMaterialLibrary))
  (bind _output_get (Variables|Default|SetMeshMaterial _returnvalue))
  ;[1 1 1] Assign material to mesh
  (Rendering|Material|SetMaterial (Variables|Default|GetStaticMesh) 0 _output_get)
  ;[1 1 1] Get base color of dynamic material
  (bind _returnvalue_2 (Rendering|Material|GetVectorParameterValue (Variables|Default|GetMeshMaterial) "BaseColor" :!class /Script/Engine.MaterialInstanceDynamic))
  (Variables|Brush|SetClearColor _returnvalue_2))

(fn CreateRenderTargets
  (bind _rendertargetsize (Variables|Default|GetRenderTargetSize))
  (bind _rendertargetsize_2 (Variables|Default|GetRenderTargetSize))
  (bind _rendertargetsize_3 (Variables|Default|GetRenderTargetSize))
  (Utilities|FlowControl|Sequence
    (:then_0
      ;[1 1 1] Create render target and assign to brush (DIFFUSE MAP)
      (bind _returnvalue (Rendering|CreateRenderTarget2D (.x _rendertargetsize_3) (.y _rendertargetsize_3) "RTF_RGBA16f"))
      (bind _output_get (Variables|Brush|SetRT _returnvalue))
      (Rendering|ClearRenderTarget2D _output_get (Variables|Brush|GetClearColor))
      (Rendering|Material|SetTextureParameterValue (Variables|Default|GetMeshMaterial) "RT" (Variables|Brush|GetRT)))
    (:then_1
      ;[1 1 1] Create render target and assign to brush (NORMAL MAP)
      (bind _returnvalue_2 (Rendering|CreateRenderTarget2D (.x _rendertargetsize) (.y _rendertargetsize) "RTF_RGBA16f"))
      (bind _output_get_2 (Variables|Brush|SetRTNormal _returnvalue_2))
      (Rendering|ClearRenderTarget2D _output_get_2 "(R=0.502887,G=0.502887,B=1.000000,A=1.000000)")
      (Rendering|Material|SetTextureParameterValue (Variables|Default|GetMeshMaterial) "RTNormal" (Variables|Brush|GetRTNormal)))
    (:then_2
      ;[1 1 1] Create render target for crack mask
      (bind _returnvalue_3 (Rendering|CreateRenderTarget2D (.x _rendertargetsize_2) (.y _rendertargetsize_2) "RTF_RGBA16f"))
      (bind _output_get_3 (Variables|Brush|SetRTCrackMask _returnvalue_3))
      (Rendering|ClearRenderTarget2D _output_get_3)
      (Rendering|Material|SetTextureParameterValue (Variables|Default|GetMeshMaterial) "RTCrackMask" (Variables|Brush|GetRTCrackMask)))))

(fn ImpactHit
  (params (OtherActor :type Actor%20Object%20Reference) (Hit :type Hit%20Result%20Structure))
  (LocalVariables|SetL_OtherActor OtherActor)
  (LocalVariables|SetL_HitImpactPoint (.ImpactPoint (Collision|BreakHitResult Hit)))
  (Update|UpdateBrushTextures)
  (Utilities|FlowControl|Sequence
    (:then_0
      ;[1 1 1] Raycast from the other actor too the impact location (FOR UV COORDINATES)
      (bind _outhits (Class|KismetSystemLibrary|LineTraceMultiforObjects (.StartPoint (Utilities|FindTraceEndPoint (Transformation|GetActorLocation (LocalVariables|GetL_OtherActor)) (LocalVariables|GetL_HitImpactPoint))) (.EndPoint (Utilities|FindTraceEndPoint (Transformation|GetActorLocation (LocalVariables|GetL_OtherActor)) (LocalVariables|GetL_HitImpactPoint))) (Utilities|Array|MakeArray "ObjectTypeQuery8") true 0 "None" false))
      ;[1 1 1] Cast each actor to this blueprint type
      (for _array_element _outhits
        (Utilities|Casting|CastToBP_SafetyGlass_DestructibleMesh_VoronoiTexture_Particle_Sound (.HitActor (Collision|BreakHitResult _array_element)))
        ;[1 1 1] Draw the material to the render targets to add broken glass
        (Rendering|Material|SetVectorParameterValue (Variables|Brush|GetGlassBrush) "Position" (Utilities|Struct|MakeLinearColor (.X (Math|Vector2D|BreakVector2D (.UV (Class|GameplayStatics|FindCollisionUV _array_element)))) (.Y (Math|Vector2D|BreakVector2D (.UV (Class|GameplayStatics|FindCollisionUV _array_element)))) 0.0 1.0) :!class /Script/Engine.MaterialInstanceDynamic)
        (Rendering|DrawMaterialtoRenderTarget (Variables|Brush|GetRT) (Variables|Brush|GetGlassBrush))
        (Rendering|Material|SetVectorParameterValue (Variables|Brush|GetGlassBrushNormal) "Position" (Utilities|Struct|MakeLinearColor (.X (Math|Vector2D|BreakVector2D (.UV (Class|GameplayStatics|FindCollisionUV _array_element)))) (.Y (Math|Vector2D|BreakVector2D (.UV (Class|GameplayStatics|FindCollisionUV _array_element)))) 0.0 1.0) :!class /Script/Engine.MaterialInstanceDynamic)
        (Rendering|DrawMaterialtoRenderTarget (Variables|Brush|GetRTNormal) (Variables|Brush|GetGlassBrushNormal))
        (Rendering|Material|SetVectorParameterValue (Variables|Brush|GetCrackBrush) "Position" (Utilities|Struct|MakeLinearColor (.X (Math|Vector2D|BreakVector2D (.UV (Class|GameplayStatics|FindCollisionUV _array_element)))) (.Y (Math|Vector2D|BreakVector2D (.UV (Class|GameplayStatics|FindCollisionUV _array_element)))) 0.0 1.0) :!class /Script/Engine.MaterialInstanceDynamic)
        (Rendering|DrawMaterialtoRenderTarget (Variables|Brush|GetRTCrackMask) (Variables|Brush|GetCrackBrush))
        (Effects|SpawnEmitteratLocation "/Game/StarterContent/Particles/P_Glass_Splintering.P_Glass_Splintering" (LocalVariables|GetL_HitImpactPoint))
        (Audio|SpawnSoundatLocation "/Game/Audio/FX/Glass/FX_Car_Window_Smash.FX_Car_Window_Smash" (LocalVariables|GetL_HitImpactPoint) "0, 0, 0" 1.0 (Math|Random|RandomFloatinRange 0.8 1.2) 0.0 0 0)))
    (:then_1
      (bind _result (Math|Integer|IncrementInt (Variables|Default|GetCurDamage))
        (:%20%20
          (if (>= _result (Variables|Default|GetMaxDamage))
            (Single|SpawnDestructibleMesh)))))))