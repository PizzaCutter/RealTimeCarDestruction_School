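; Safety glass actor that accumulates randomized impact decals where other objects hit its mesh.
; BeginPlay creates color and normal render targets for the dynamic mesh material, plus brush materials to draw into them.
; On hit, a complex multi-trace extended past the impact finds glass surfaces, and brushes paint at their collision UVs.
; Voronoi and high-pass textures are baked to shared render targets during construction and BeginPlay.
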(event OnComponentHit(StaticMesh)
  (params (HitComponent :type Primitive%20Component%20Object%20Reference) (OtherActor :type Actor%20Object%20Reference) (OtherComp :type Primitive%20Component%20Object%20Reference) (NormalImpulse :type Vector :default "0, 0, 0") (Hit :type Hit%20Result%20Structure%20%28by%20ref%29))
  (bind _returnvalue (Transformation|GetActorLocation OtherActor))
  (CallFunction|UpdateDecals)
  (bind _outhits (Class|KismetSystemLibrary|LineTraceMultiforObjects _returnvalue (+ (.impactpoint Hit) (* (Math|Vector|Normalize (- (.impactpoint Hit) _returnvalue)) (Variables|Default|GetAdditionalRaycastLength))) (Utilities|Array|MakeArray "ObjectTypeQuery2" "ObjectTypeQuery1" "ObjectTypeQuery5") true 0 "None" false))
  (for _array_element _outhits
    (Utilities|Casting|CastToBP_SafetyGlass (.HitActor (Collision|BreakHitResult _array_element)))
    (Rendering|Material|SetVectorParameterValue (Variables|Default|GetGlassBrush) "Position" (Utilities|Struct|MakeLinearColor (.X (Math|Vector2D|BreakVector2D (.UV (Class|GameplayStatics|FindCollisionUV _array_element)))) (.Y (Math|Vector2D|BreakVector2D (.UV (Class|GameplayStatics|FindCollisionUV _array_element)))) 0.0 1.0) :!class /Script/Engine.MaterialInstanceDynamic)
    (Rendering|DrawMaterialtoRenderTarget (Variables|Default|GetRT) (Variables|Default|GetGlassBrush))
    (Rendering|Material|SetVectorParameterValue (Variables|Default|GetGlassBrushNormal) "Position" (Utilities|Struct|MakeLinearColor (.X (Math|Vector2D|BreakVector2D (.UV (Class|GameplayStatics|FindCollisionUV _array_element)))) (.Y (Math|Vector2D|BreakVector2D (.UV (Class|GameplayStatics|FindCollisionUV _array_element)))) 0.0 1.0) :!class /Script/Engine.MaterialInstanceDynamic)
    (Rendering|DrawMaterialtoRenderTarget (Variables|Default|GetRTNormal) (Variables|Default|GetGlassBrushNormal))))

(event EventBeginPlay
  (bind _rendertargetsize (Variables|Default|GetRenderTargetSize))
  (bind _rendertargetsize_2 (Variables|Default|GetRenderTargetSize))
  (Utilities|FlowControl|Sequence
    (:then_0
      ;[1 1 1] Create brush material
      (bind _returnvalue (Rendering|Material|CreateDynamicMaterialInstance "/Game/Materials/SafetyGlass/Brushes/M_GlassBrush.M_GlassBrush" "None" :!class /Script/Engine.KismetMaterialLibrary))
      (bind _output_get (Variables|Default|SetGlassBrush _returnvalue))
      (Rendering|Material|SetScalarParameterValue _output_get "Size" (Variables|Default|GetBrushSize) :!class /Script/Engine.MaterialInstanceDynamic)
      ;[1 1 1] Create brush for normal maps
      (bind _returnvalue_2 (Rendering|Material|CreateDynamicMaterialInstance "/Game/Materials/SafetyGlass/Brushes/M_GlassBrushNormal.M_GlassBrushNormal" "None" :!class /Script/Engine.KismetMaterialLibrary))
      (bind _output_get_2 (Variables|Default|SetGlassBrushNormal _returnvalue_2))
      (Rendering|Material|SetScalarParameterValue _output_get_2 "Size" (Variables|Default|GetBrushSize) :!class /Script/Engine.MaterialInstanceDynamic)
      ;[1 1 1] Create glass material for static mesh
      (bind _returnvalue_3 (Rendering|Material|CreateDynamicMaterialInstance (Rendering|Material|GetMaterial (Variables|Default|GetStaticMesh) 0) "None" :!class /Script/Engine.KismetMaterialLibrary))
      (bind _output_get_3 (Variables|Default|SetMeshMaterial _returnvalue_3))
      (Rendering|Material|SetMaterial (Variables|Default|GetStaticMesh) 0 _output_get_3)
      (bind _returnvalue_4 (Rendering|Material|GetVectorParameterValue (Variables|Default|GetMeshMaterial) "BaseColor" :!class /Script/Engine.MaterialInstanceDynamic))
      (Variables|Default|SetClearColor _returnvalue_4))
    (:then_1
      ;[1 1 1] Create render target and assign it to the brush
      (bind _returnvalue_5 (Rendering|CreateRenderTarget2D (.x _rendertargetsize_2) (.y _rendertargetsize_2) "RTF_RGBA16f"))
      (bind _output_get_4 (Variables|Default|SetRT _returnvalue_5))
      (Rendering|ClearRenderTarget2D _output_get_4 (Variables|Default|GetClearColor))
      (Rendering|Material|SetTextureParameterValue (Variables|Default|GetMeshMaterial) "RT" (Variables|Default|GetRT)))
    (:then_2
      (bind _returnvalue_6 (Rendering|CreateRenderTarget2D (.x _rendertargetsize) (.y _rendertargetsize) "RTF_RGBA16f"))
      (bind _output_get_5 (Variables|Default|SetRTNormal _returnvalue_6))
      (Rendering|ClearRenderTarget2D _output_get_5 "(R=0.502887,G=0.502887,B=1.000000,A=1.000000)")
      (Rendering|Material|SetTextureParameterValue (Variables|Default|GetMeshMaterial) "RTNormal" (Variables|Default|GetRTNormal)))
    (:then_3
      (CallFunction|BakeVoronoi))))

(fn ConstructionScript
  (CallFunction|BakeVoronoi))

(fn UpdateDecals
  (bind _brushtextures (Variables|Default|GetBrushTextures))
  (bind _brushnormaltextures (Variables|Default|GetBrushNormalTextures))
  (Rendering|Material|SetTextureParameterValue (Variables|Default|GetGlassBrush) "Decal" (Utilities|Array|Get(acopy) _brushtextures (Math|Random|RandomInteger (Utilities|Array|Length _brushtextures))))
  (Rendering|Material|SetTextureParameterValue (Variables|Default|GetGlassBrushNormal) "Decal" (Utilities|Array|Get(acopy) _brushnormaltextures (Math|Random|RandomInteger (Utilities|Array|Length _brushnormaltextures)))))

(fn BakeVoronoi
  (Rendering|DrawMaterialtoRenderTarget "/Game/Blueprints/SafetyGlass/RT_Voronoi.RT_Voronoi" "/Game/Materials/SafetyGlass/Voronoi/M_Voronoi.M_Voronoi")
  (Rendering|DrawMaterialtoRenderTarget "/Game/Blueprints/SafetyGlass/RT_Voronoi_HighPass.RT_Voronoi_HighPass" "/Game/Materials/SafetyGlass/Voronoi/M_Voronoi_HighPass.M_Voronoi_HighPass")
  (Rendering|DrawMaterialtoRenderTarget "/Game/Blueprints/SafetyGlass/RT_Voronoi_HighPass_Normal.RT_Voronoi_HighPass_Normal" "/Game/Materials/SafetyGlass/Voronoi/M_Voronoi_HighPass_Normal.M_Voronoi_HighPass_Normal"))