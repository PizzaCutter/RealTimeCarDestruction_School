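; Free-flying player pawn that looks around with the mouse and launches physics balls from the camera, under an object denting section.
; Axis inputs and gated raise/lower actions feed FloatingPawnMovement, while Tick drives the vertical gates and clamps camera pitch with roll zeroed.
; Shoot spawns the Throwable class and applies a velocity-change impulse along the camera's forward vector.
; A line-trace dent placement branch with debug drawing is left unconnected.
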(event Custom|RaiseTick
  ;[0.7365 1 0] MOVEMENT CODE
  (Utilities|FlowControl|Gate true
    (:Exit
      (Class|PawnMovementComponent|AddInputVector (Variables|Default|GetFloatingPawnMovement) (* "0, 0,1.000000" 1.0) false))))

(event Custom|LowerTick
  ;[0.7365 1 0] MOVEMENT CODE
  (Utilities|FlowControl|Gate true
    (:Exit
      (Class|PawnMovementComponent|AddInputVector (Variables|Default|GetFloatingPawnMovement) (* "0, 0,1.000000" -1.0) false))))

(event EventTick
  (params (DeltaSeconds :type Float%20%28single-precision%29))
  (CallFunction|ClampRotation)
  (CallFunction|RaiseTick)
  (CallFunction|LowerTick))

(event Input|ActionEvents|InputActionShoot
  (params (Key :type Key%20Structure))
  (:Pressed
    (bind _returnvalue (Game|SpawnActorfromClass (Variables|Default|GetThrowable) (Transformation|GetWorldTransform (Variables|Default|GetCamera)) "AlwaysSpawn" 0 0))
    (bind _asphysics_ball (Utilities|Casting|CastToPhysicsBall _returnvalue))
    (Physics|AddImpulse (Variables|/Game/Blueprints/Throwables/PhysicsBall.PhysicsBall_C|GetSphere _asphysics_ball) (* (Math|Vector|GetForwardVector (Variables|Default|GetCamera)) (Variables|Default|GetThrowVelocity)) "None" true)))

(event Input|ActionEvents|InputActionRaise
  (params (Key :type Key%20Structure))
  ;[0.7365 1 0] MOVEMENT CODE
  (:Pressed
    (Utilities|FlowControl|Gate true) ; enters at Open
  )
  (:Released
    (Utilities|FlowControl|Gate true) ; enters at Close
  ))

(event Input|ActionEvents|InputActionLower
  (params (Key :type Key%20Structure))
  ;[0.7365 1 0] MOVEMENT CODE
  (:Pressed
    (Utilities|FlowControl|Gate true) ; enters at Open
  )
  (:Released
    (Utilities|FlowControl|Gate true) ; enters at Close
  ))

(event Input|AxisEvents|InputAxisHorizontal
  (params (AxisValue :type Float%20%28single-precision%29))
  ;[0.7365 1 0] MOVEMENT CODE
  (Class|PawnMovementComponent|AddInputVector (Variables|Default|GetFloatingPawnMovement) (* (Math|Vector|GetForwardVector (Variables|Default|GetCamera)) AxisValue) false))

(event Input|AxisEvents|InputAxisVertical
  (params (AxisValue :type Float%20%28single-precision%29))
  ;[0.7365 1 0] MOVEMENT CODE
  (Class|PawnMovementComponent|AddInputVector (Variables|Default|GetFloatingPawnMovement) (* (Math|Vector|GetRightVector (Variables|Default|GetCamera)) AxisValue) false))

(event Input|AxisEvents|InputAxisMouseHorizontal
  (params (AxisValue :type Float%20%28single-precision%29))
  ;[0.7365 1 0] MOVEMENT CODE
  (Transformation|AddRelativeRotation (Variables|Default|GetCamera) (Math|Rotator|MakeRotator 0.0 0.0 AxisValue) false false))

(event Input|AxisEvents|InputAxisMouseVertical
  (params (AxisValue :type Float%20%28single-precision%29))
  ;[0.7365 1 0] MOVEMENT CODE
  (Transformation|AddRelativeRotation (Variables|Default|GetCamera) (Math|Rotator|MakeRotator 0.0 AxisValue 0.0) false false))

(event Input|MouseEvents|RightMouseButton
  (params (Key :type Key%20Structure))
  ;[1 0 0.5677] OBJECT DENTING
)

(fn ConstructionScript)

(fn ClampRotation
  (bind _camera (Variables|Default|GetCamera))
  (bind _returnvalue (Transformation|GetWorldRotation _camera))
  (Transformation|SetWorldRotation (Variables|Default|GetCamera) (Math|Rotator|MakeRotator 0.0 (Math|Float|ClampAngle (.pitch _returnvalue) -8e+01 8e+01) (Class|KismetMathLibrary|ClampAxis (.yaw _returnvalue))) false false))