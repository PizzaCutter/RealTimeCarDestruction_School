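; Dentable mesh actor that records hard impacts as dents in its material and destroys the actor that hit it.
; Construction creates a nearest-filtered render target and binds it, with radius and offset settings, to a dynamic M_DentFromRT material.
; Each qualifying hit writes the other actor's location and the impact normal into consecutive pixels, wrapping to overwrite from the start when full.
; An optional plane previews the render target.
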(event OnComponentHit(Mesh)
  (params (HitComponent :type Primitive%20Component%20Object%20Reference) (OtherActor :type Actor%20Object%20Reference) (OtherComp :type Primitive%20Component%20Object%20Reference) (NormalImpulse :type Vector :default "0, 0, 0") (Hit :type Hit%20Result%20Structure%20%28by%20ref%29))
  (if (> (Math|Vector|VectorLength NormalImpulse) (Variables|Constructor|GetMinImpactRequired))
    (bind (_canvas _size _context) (Rendering|BeginDrawCanvastoRenderTarget (Variables|UsedInternally|GetRT)))
    (Canvas|DrawTexture :self _canvas :ScreenPosition (Math|Vector2D|MakeVector2D (Math|Conversions|ToFloat(Integer) (Variables|UsedInternally|GetXIndex)) (Math|Conversions|ToFloat(Integer) (Variables|UsedInternally|GetYIndex))) :ScreenSize "(X=1.000000,Y=1.000000)" :RenderColor (Math|Conversions|ToLinearColor(Vector) (Transformation|GetActorLocation OtherActor)) :BlendMode "BLEND_Opaque" :PivotPoint "(X=0.500000,Y=0.500000)")
    (CallFunction|UpdateIndex)
    (Canvas|DrawTexture :self _canvas :ScreenPosition (Math|Vector2D|MakeVector2D (Math|Conversions|ToFloat(Integer) (Variables|UsedInternally|GetXIndex)) (Math|Conversions|ToFloat(Integer) (Variables|UsedInternally|GetYIndex))) :ScreenSize "(X=1.000000,Y=1.000000)" :RenderColor (Math|Conversions|ToLinearColor(Vector) (.impactnormal Hit)) :BlendMode "BLEND_Opaque" :PivotPoint "(X=0.500000,Y=0.500000)")
    (CallFunction|UpdateIndex)
    (Rendering|EndDrawCanvastoRenderTarget _context)
    (Actor|DestroyActor OtherActor)))

(event EventBeginPlay
  (CallFunction|ClearRenderTarget))

(fn ConstructionScript
  (CallFunction|InitializeDentableMesh))

(fn UpdateIndex
  (Utilities|FlowControl|Sequence
    (:then_0
      (bind _result (Math|Integer|IncrementInt (Variables|UsedInternally|GetXIndex))
        (:%20%20
          (if (>= _result (.x (Variables|Constructor|GetRT_Dimensions)))
            (Variables|UsedInternally|SetXIndex 0)
            (Math|Integer|IncrementInt (Variables|UsedInternally|GetYIndex))))))
    (:then_1
      (if (>= (Variables|UsedInternally|GetYIndex) (.y (Variables|Constructor|GetRT_Dimensions)))
        (Variables|UsedInternally|SetXIndex 0)
        (Variables|UsedInternally|SetYIndex 0)))))

(fn InitializeDentableMesh
  (bind _rt_dimensions (Variables|Constructor|GetRT_Dimensions))
  (Utilities|FlowControl|Sequence
    (:then_0
      ;[1 1 1] Create render target to save dent position data
      (bind _returnvalue (CanvasRenderTarget2D|CreateCanvasRenderTarget2D "/Game/Blueprints/MaterialDeformation/RT_Dent.RT_Dent_C" (.x _rt_dimensions) (.y _rt_dimensions)))
      (bind _asrt_dent (Utilities|Casting|CastToRT_Dent _returnvalue))
      (bind _output_get (Variables|UsedInternally|SetRT _asrt_dent))
      (Variables|/Script/Engine.Texture|SetFilter _output_get "TF_Nearest")
      (CallFunction|ClearRenderTarget))
    (:then_1
      ;[1 1 1] Create dynamic material and set parameter values for denting
      (bind _returnvalue_2 (Rendering|Material|CreateDynamicMaterialInstance "/Game/Materials/MaterialDeformation/M_DentFromRT.M_DentFromRT" "None" :!class /Script/Engine.KismetMaterialLibrary))
      (LocalVariables|SetDynamicMaterial _returnvalue_2)
      (Rendering|Material|SetMaterial (Variables|Default|GetMesh) 0 (LocalVariables|GetDynamicMaterial))
      (Rendering|Material|SetTextureParameterValue (LocalVariables|GetDynamicMaterial) "DentLocations" (Variables|UsedInternally|GetRT))
      (Rendering|Material|SetScalarParameterValue (LocalVariables|GetDynamicMaterial) "Width" (Math|Conversions|ToFloat(Integer) (.x (Variables|Constructor|GetRT_Dimensions))) :!class /Script/Engine.MaterialInstanceDynamic)
      (Rendering|Material|SetScalarParameterValue (LocalVariables|GetDynamicMaterial) "Height" (Math|Conversions|ToFloat(Integer) (.y (Variables|Constructor|GetRT_Dimensions))) :!class /Script/Engine.MaterialInstanceDynamic)
      (Rendering|Material|SetScalarParameterValue (LocalVariables|GetDynamicMaterial) "DentRadius" (Variables|Constructor|GetDentRadius) :!class /Script/Engine.MaterialInstanceDynamic)
      (Rendering|Material|SetVectorParameterValue (LocalVariables|GetDynamicMaterial) "MinOffset" (Math|Conversions|ToLinearColor(Vector) (Variables|Constructor|GetMinOffset)) :!class /Script/Engine.MaterialInstanceDynamic)
      (Rendering|Material|SetVectorParameterValue (LocalVariables|GetDynamicMaterial) "MaxOffset" (Math|Conversions|ToLinearColor(Vector) (Variables|Constructor|GetMaxOffset)) :!class /Script/Engine.MaterialInstanceDynamic))
    (:then_2
      ;[1 1 1] Enable/Disable previewing render target on a plane
      (if (Variables|Constructor|GetPreviewRenderTarget)
        (bind _returnvalue_3 (Rendering|Material|CreateDynamicMaterialInstance 0 "None" :!class /Script/Engine.KismetMaterialLibrary))
        (bind _output_get_2 (LocalVariables|SetDynamicMaterial _returnvalue_3))
        (Rendering|Material|SetTextureParameterValue _output_get_2 "RT" (Variables|UsedInternally|GetRT))
        (Rendering|Material|SetMaterial (Variables|Default|GetRenderTargetPreview) 0 (LocalVariables|GetDynamicMaterial))
        (Rendering|SetVisibility (Variables|Default|GetRenderTargetPreview) true false)))))

(fn ClearRenderTarget
  (Rendering|ClearRenderTarget2D (Variables|UsedInternally|GetRT)))